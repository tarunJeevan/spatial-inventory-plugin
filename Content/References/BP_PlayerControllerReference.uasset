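; Player controller that owns the inventory screen and handles its input.
; On BeginPlay it adds the inventory input mapping context and creates the inventory widget from the class set on the player character's InventoryComponent.
; The inventory action toggles the widget in the viewport, switching mouse cursor and input mode with it.
; The rotate action forwards to the inventory grid widget to rotate the dragged item.
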(event Input|EnhancedActionEvents|EnhancedInputActionIA_Inventory
  (params (ActionValue :type Boolean) (ElapsedSeconds :type Float%20%28double-precision%29) (TriggeredSeconds :type Float%20%28double-precision%29) (InputAction :type Input%20Action%20Object%20Reference :default "/SpatialInventory/Input/IA_Inventory.IA_Inventory"))
  (bind _inventorywidget (Variables|Default|GetInventoryWidget))
  (if (UserInterface|Viewport|IsinViewport (Variables|Default|GetInventoryWidget))
    (Widget|RemovefromParent (Variables|Default|GetInventoryWidget))
    (Variables|Default|SetbShowMouseCursor false)
    (Input|SetInputModeGameOnly self false)
    (else
      (UserInterface|Viewport|AddtoViewport _inventorywidget 0)
      (Variables|Default|SetbShowMouseCursor true)
      (Input|SetInputModeGameandUI self _inventorywidget "DoNotLock" false false))))

(event Input|EnhancedActionEvents|EnhancedInputActionIA_RotateItem
  (params (ActionValue :type Boolean) (ElapsedSeconds :type Float%20%28double-precision%29) (TriggeredSeconds :type Float%20%28double-precision%29) (InputAction :type Input%20Action%20Object%20Reference :default "/SpatialInventory/Input/IA_RotateItem.IA_RotateItem"))
  (Class|InventoryGridWidget|RotateDraggedItem (Class|InventoryWidget|GetInventoryGridWidget (Variables|Default|GetInventoryWidget))))

(event EventBeginPlay
  (Input|AddMappingContext (PlayerController|LocalPlayerSubsystems|GetEnhancedInputLocalPlayerSubsystem self) "/SpatialInventory/Input/IMC_Inventory.IMC_Inventory" 1 "(bIgnoreAllPressedKeysUntilRelease=True,bForceImmediately=False,bNotifyUserSettings=False)")
  (bind _asbp_player_character (Utilities|Casting|CastToBP_PlayerCharacter (Game|Player|GetPlayerPawn 0)))
  (bind _returnvalue (UserInterface|CreateWidget (Variables|/Script/SpatialInventory.InventoryComponent|GetInventoryWidgetClass (Variables|/Script/PluginTestBed.CustomCharacter|GetInventoryComponent _asbp_player_character)) self))
  (bind _aswbp_inventory_widget (Utilities|Casting|CastToWBP_InventoryWidget _returnvalue))
  (Variables|Default|SetInventoryWidget _aswbp_inventory_widget))

(fn ConstructionScript)